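; Bystander_Stander is a bystander actor that randomly thins and varies its placed instances when play begins.
; After calling the parent BeginPlay, it usually destroys itself on a weighted random roll, so only a minority of instances remain.
; Survivors receive a small random yaw offset in either direction to vary their facing.
; The construction script only calls the parent, and the overlap and tick events are disabled stubs.
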(event `self.ReceiveBeginPlay`
  (`parent.ReceiveBeginPlay`)
  (if (`KismetMathLibrary.RandomBoolWithWeight` 0.7)
    (`self.K2_DestroyActor`)
    (else
      (`self.K2_AddActorWorldRotation` (`KismetMathLibrary.MakeRotator` 0.0 0.0 (`KismetMathLibrary.RandomFloatInRange` -30.0 30.0))))))

(fn `UserConstructionScript`
  (`parent.UserConstructionScript`))