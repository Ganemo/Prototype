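; Two-player bounce wall that relaunches a ball on contact and carries a score widget for each of two players.
; At BeginPlay, its two widget components' ScoreWidgets are bound to target characters 0 and 1.
; When ball contact begins, it flags the ball as having hit a wall, calls LaunchBall with the ball's current velocity and plays a bounce sound at the wall's location.
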(event `self.ReceiveBeginPlay`
  (bind _asscore_widget (cast `/Game/UI/ScoreWidget` (`WidgetComponent.GetUserWidgetObject` (`self.Widget`))))
  (set `/Game/UI/ScoreWidget.TargetCharacter` 0 _asscore_widget)
  (bind _asscore_widget_2 (cast `/Game/UI/ScoreWidget` (`WidgetComponent.GetUserWidgetObject` (`self.Widget1`))))
  (set `/Game/UI/ScoreWidget.TargetCharacter` 1 _asscore_widget_2))

(event `self.ContactWithBall_Begin`
  (params (ball :type "Ball Object Reference"))
  (set `Ball.bHitWall` true ball)
  (`Ball.LaunchBall` ball (`self.GetVelocity` ball))
  (`GameplayStatics.PlaySoundAtLocation` "/Game/Audio/BallBounce_Cue.BallBounce_Cue" (`self.K2_GetActorLocation`)))

(fn `UserConstructionScript`)