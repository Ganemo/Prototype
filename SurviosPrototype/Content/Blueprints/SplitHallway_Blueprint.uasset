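; Split hallway actor that bounces the ball along the X axis when the ball makes contact with it.
; On contact it plays a bounce sound at the ball's location and relaunches the ball along its normalized velocity with an adjusted X.
; The ball's HitWall flag forces X negative when set and positive otherwise, leaving Y and Z unchanged.
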(event `self.ContactWithBall_Begin`
  (params (ball :type "Ball Object Reference"))
  (bind _returnvalue (`KismetMathLibrary.Normal` (`self.GetVelocity` ball)))
  (`GameplayStatics.PlaySoundAtLocation` "/Game/Audio/BallBounce_Cue.BallBounce_Cue" (`self.K2_GetActorLocation` ball))
  (if (`Ball.bHitWall` ball)
    (`Ball.LaunchBall` ball (`KismetMathLibrary.MakeVector` (* (`KismetMathLibrary.Abs` (.x _returnvalue)) -1.0) (.y _returnvalue) (.z _returnvalue)))
    (else
      (`Ball.LaunchBall` ball (`KismetMathLibrary.MakeVector` (`KismetMathLibrary.Abs` (.x _returnvalue)) (.y _returnvalue) (.z _returnvalue))))))

(fn `UserConstructionScript`)