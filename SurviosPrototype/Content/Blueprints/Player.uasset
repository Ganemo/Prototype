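; Player character for a racket ball game that walks in, has PaddleGameMode spawn a ball, then swings at it.
; IsLefty selects the racket socket, side spring arm offset and montages.
; Swings enable RacketHit collision only while the montage plays and block re-swinging until it completes.
; Ball contact strikes the ball, plays a ping and starts per-tick camera work, easing arm length from hip movement and rotation toward the ball.
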(event `self.Init`
  (bind _racket (`self.Racket`))
  (bind _mesh (`self.Mesh`))
  (bind _mesh_2 (`self.Mesh`))
  (bind _springarm1 (`self.SpringArm1`))
  (`SkeletalMeshComponent.SetAnimInstanceClass` (`self.Mesh`) "/Game/Animations/Player_AnimBP.Player_AnimBP_C")
  (set `self.bCanSwing` false)
  (if (`self.bIsLefty`)
    (`SceneComponent.K2_AttachToComponent` _racket _mesh "RacketSocket_L" "KeepRelative" "KeepRelative" "KeepRelative" true)
    (set `SpringArmComponent.TargetArmLength` 100.0 _springarm1)
    (`|PlayMontage` _mesh_2 "/Game/Animations/Baseball_Walk_In_Montage.Baseball_Walk_In_Montage"
      (:`OnCompleted`
        _))
    (else
      (`SceneComponent.K2_AttachToComponent` _racket _mesh "RacketSocket_R" "KeepRelative" "KeepRelative" "KeepRelative" true)
      (set `SpringArmComponent.TargetArmLength` -100.0 _springarm1)
      (`|PlayMontage` _mesh_2 "/Game/Animations/Baseball_Walk_In_Inv_Montage.Baseball_Walk_In_Inv_Montage"
        (:`OnCompleted`
          _))))
  (`KismetSystemLibrary.Delay` 0.2)
  (bind _aspaddle_game_mode (cast `PaddleGameMode` (`GameplayStatics.GetGameMode`)))
  (`PaddleGameMode.SpawnBall` _aspaddle_game_mode)
  (set `self.bCanSwing` true))

(event `self.ReceiveTick`
  (params (DeltaSeconds :type "Float (single-precision)"))
  (if (`self.bDoCameraWork`)
    (`self.DoCameraShifting` DeltaSeconds
      (:` `
        (`self.DoBallFocus` DeltaSeconds)))))

(event `self.Swing`
  (bind _mesh (`self.Mesh`))
  (if (`self.bCanSwing`)
    (if (`self.bIsLefty`)
      (`|PlayMontage` _mesh "/Game/Animations/Baseball_Swing.Baseball_Swing"
        (:`then`
          (`self.SetPaddleState` true :!label _label))
        (:`OnCompleted`
          (`self.SetPaddleState` false :!label _label_2)))
      (else
        (`|PlayMontage` _mesh "/Game/Animations/Baseball_Hit_Inv_Montage.Baseball_Hit_Inv_Montage"
          (:`then`
            (goto _label))
          (:`OnCompleted`
            (goto _label_2)))))))

(event `self.ContactWithBall_Begin`
  (params (ball :type "Ball Object Reference"))
  (`self.StrikeBall` ball)
  (set `self.Ball` ball)
  (set `self.bDoCameraWork` true)
  (`GameplayStatics.PlaySoundAtLocation` "/Game/Audio/BallPing_Cue.BallPing_Cue" (`self.K2_GetActorLocation` ball)))

(event `self.SetPaddleState`
  (params (NewState :type Boolean))
  (bind _rackethit (`self.RacketHit`))
  (if NewState
    (set `self.bCanSwing` false)
    (set `self.bActiveSwing` true)
    (`PrimitiveComponent.SetCollisionEnabled` _rackethit "QueryOnly")
    (else
      (set `self.bCanSwing` true)
      (set `self.bActiveSwing` false)
      (`PrimitiveComponent.SetCollisionEnabled` _rackethit "NoCollision"))))

(fn `UserConstructionScript`
  (`parent.UserConstructionScript`))